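; Board logic Blueprint that builds a hexagon-style game board of BoardSpheres actors at BeginPlay.
; SpawnCircle runs per ring index up to SizeOfBoard, placing a centre sphere, then rings based on six times the ring number.
; Trigonometry places corners at 60-degree multiples on full radius; spheres between use HexConst plus an accumulating HexDiffEnd correction to approximate straight edges.
; Debug prints of the correction and angle values remain.
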(event EventBeginPlay
  (for _index (range 0 (Variables|Default|GetsizeOfBoard))
    (CallFunction|SpawnCircle 0.0 0.0 0.0 _index)))

(event Collision|EventActorBeginOverlap
  (params (OtherActor :type Actor%20Object%20Reference)))

(event EventTick
  (params (DeltaSeconds :type Float%20%28single-precision%29)))

(fn ConstructionScript)

(fn SpawnCircle
  (params (X :type Float%20%28double-precision%29) (Y :type Float%20%28double-precision%29) (Z :type Float%20%28double-precision%29) (Num :type Integer))
  (bind _returnvalue (Math|Vector|MakeVector X Y Z))
  (bind _returnvalue_2 (- Num 1))
  (bind _returnvalue_3 (* Num 6))
  (bind _sizeofcircles (Variables|Default|GetsizeOfCircles))
  (bind _hexconst (Variables|Default|GetHexConst))
  (bind _sizeofcircles_2 (Variables|Default|GetsizeOfCircles))
  (bind _sizeofcircles_3 (Variables|Default|GetsizeOfCircles))
  (bind _sizeofcircles_4 (Variables|Default|GetsizeOfCircles))
  (bind _sizeofcircles_5 (Variables|Default|GetsizeOfCircles))
  (Variables|Default|SetHexDiff (- 1.0 (Variables|Default|GetHexConst)))
  (if (== Num 0)
    (Game|SpawnActorfromClass "/Game/Objects/boardSpheres.boardSpheres_C" (Math|Transform|MakeTransform _returnvalue "0, 0, 0" (Math|Vector|MakeVector _sizeofcircles_4 _sizeofcircles_4 _sizeofcircles_4)) "Undefined" 0 0)
    (else
      (if (<= _returnvalue_2 1)
        _
        (else
          (bind _output_get (Variables|Default|SetHexDiffEnd (+ (Variables|Default|GetHexDiffEnd) (/ (Variables|Default|GetHexDiff) (* 6.0 _returnvalue_2)))))
          (Development|PrintText (Utilities|Text|ToText(Float) _output_get "HalfToEven"))))
      (for _index (range 0 _returnvalue_3)
        (if (== (Math|Float|%(Float) (* _index (/ (Variables|Default|Getdegrees) (Math|Conversions|ToFloat(Integer) _returnvalue_3))) 6e+01) 0.0)
          (Game|SpawnActorfromClass "/Game/Objects/boardSpheres.boardSpheres_C" (Math|Transform|MakeTransform (+ _returnvalue (* (* (Math|Vector|MakeVector (Math|Trig|Cos(Degrees) (* _index (/ (Variables|Default|Getdegrees) (Math|Conversions|ToFloat(Integer) _returnvalue_3)))) (Math|Trig|Sin(Degrees) (* _index (/ (Variables|Default|Getdegrees) (Math|Conversions|ToFloat(Integer) _returnvalue_3)))) 0.0) (* Num _sizeofcircles_5)) (Variables|Default|GetworldScale))) "0, 0, 0" (Math|Vector|MakeVector _sizeofcircles_5 _sizeofcircles_5 _sizeofcircles_5)) "Undefined" 0 0)
          (else
            (Development|PrintText "Cos")
            (Development|PrintText (Utilities|Text|ToText(Float) (Math|Trig|Cos(Degrees) (* _index (/ (Variables|Default|Getdegrees) (Math|Conversions|ToFloat(Integer) _returnvalue_3)))) "HalfToEven"))
            (Development|PrintText "Sin")
            (Development|PrintText (Utilities|Text|ToText(Float) (Math|Trig|Sin(Degrees) (* _index (/ (Variables|Default|Getdegrees) (Math|Conversions|ToFloat(Integer) _returnvalue_3)))) "HalfToEven"))
            (Game|SpawnActorfromClass "/Game/Objects/boardSpheres.boardSpheres_C" (Math|Transform|MakeTransform (+ _returnvalue (* (* (Math|Vector|MakeVector (* (* (Math|Trig|Cos(Degrees) (* _index (/ (Variables|Default|Getdegrees) (Math|Conversions|ToFloat(Integer) _returnvalue_3)))) _hexconst) _sizeofcircles_2) (* (* (Math|Trig|Sin(Degrees) (* _index (/ (Variables|Default|Getdegrees) (Math|Conversions|ToFloat(Integer) _returnvalue_3)))) _hexconst) _sizeofcircles_2) 0.0) (* Num _sizeofcircles_2)) (Variables|Default|GetworldScale)) (* (* (Math|Vector|MakeVector (* (* (Math|Trig|Cos(Degrees) (* _index (/ (Variables|Default|Getdegrees) (Math|Conversions|ToFloat(Integer) _returnvalue_3)))) (Variables|Default|GetHexDiffEnd)) _sizeofcircles_3) (* (* (Math|Trig|Sin(Degrees) (* _index (/ (Variables|Default|Getdegrees) (Math|Conversions|ToFloat(Integer) _returnvalue_3)))) (Variables|Default|GetHexDiffEnd)) _sizeofcircles_3) 0.0) (* _sizeofcircles_3 Num)) (Variables|Default|GetworldScale))) "0, 0, 0" (Math|Vector|MakeVector _sizeofcircles _sizeofcircles _sizeofcircles)) "Undefined" 0 0)))))))